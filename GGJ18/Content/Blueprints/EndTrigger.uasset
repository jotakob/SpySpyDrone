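; EndTrigger is a goal trigger actor that wins the game when two players are inside it.
; It increments PlayersInGoal when a TopDownCharacter begins overlapping and decrements it when one leaves.
; When the count reaches two, it casts the game mode to TopDownGameMode and calls WinGame.
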(event `self.ReceiveActorBeginOverlap`
  (params (OtherActor :type "Actor Object Reference"))
  (cast `/Game/Actors/Character/TopDownCharacter` OtherActor)
  (bind _result (`/Engine/EditorBlueprintResources/StandardMacros.IncrementInt` (`self.PlayersInGoal`))
    (:`  `
      (if (== _result 2)
        (bind _astop_down_game_mode (cast `/Game/Blueprints/TopDownGameMode` (`GameplayStatics.GetGameMode`)))
        (`/Game/Blueprints/TopDownGameMode.WinGame` _astop_down_game_mode)))))

(event `self.ReceiveActorEndOverlap`
  (params (OtherActor :type "Actor Object Reference"))
  (cast `/Game/Actors/Character/TopDownCharacter` OtherActor)
  (`/Engine/EditorBlueprintResources/StandardMacros.DecrementInt` (`self.PlayersInGoal`)))

(fn `UserConstructionScript`)